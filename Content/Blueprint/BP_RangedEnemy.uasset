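; BP_RangedEnemy is a ranged enemy, apparently derived from a Goblin Blueprint, that attacks by launching fireballs.
; Its Attack event plays the attack montage, then immediately spawns a BP_Fireball at the ProjectileSpawnPos transform, always spawning regardless of collision.
; The enemy passes its Damaged value to each new fireball.
; BeginPlay, overlap and Tick events are disabled stubs, and the graph holds no other logic.
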(event `self.Attack`
  (`self.PlayAnimMontage` (`self.AttackAnimation`))
  (bind _returnvalue (`|SpawnActorFromClass` "/Game/Blueprint/BP_Fireball.BP_Fireball_C" (`SceneComponent.K2_GetComponentToWorld` (`self.ProjectileSpawnPos`)) "AlwaysSpawn" "MultiplyWithRoot" null null))
  (set `/Game/Blueprint/BP_Fireball.Damaged` (`self.Damaged`) _returnvalue))

(fn `UserConstructionScript`
  (`parent.UserConstructionScript`))