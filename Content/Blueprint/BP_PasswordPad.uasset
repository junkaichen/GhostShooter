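; BP_PasswordPad is an interactable keypad actor that opens a password entry UI to unlock a door.
; At BeginPlay it pre-creates a prompt widget and a pad widget, passing the pad itself and an IsFirstDoor flag.
; Its box overlap shows or hides the prompt and sets an in-range flag that gates Interact, which switches to UI-only input with a cursor.
; UnlockSecondDoor destroys the linked PasswordDoor actor.
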(event `self.ReceiveBeginPlay`
  (bind _returnvalue (`|CreateWidget` "/Game/UI/BPW_Prompt.BPW_Prompt_C"))
  (set `self.PromptUI` _returnvalue)
  (bind _returnvalue_2 (`|CreateWidget` "/Game/UI/BPW_PassWordPad.BPW_PassWordPad_C" null (`self.IsFirstDoor`) self))
  (set `self.PasswordPadUI` _returnvalue_2))

(event `self.Box.OnComponentBeginOverlap`
  (params (OverlappedComponent :type "PrimitiveComponent Object Reference") (OtherActor :type "Actor Object Reference") (OtherComp :type "PrimitiveComponent Object Reference") (OtherBodyIndex :type Integer) (bFromSweep :type Boolean) (SweepResult :type "HitResult Structure (by ref)"))
  (set `self.IsInInteractableRange` true)
  (if (== OtherActor (`GameplayStatics.GetPlayerCharacter` 0))
    (`UserWidget.AddToViewport` (`self.PromptUI`) 0)))

(event `self.Box.OnComponentEndOverlap`
  (params (OverlappedComponent :type "PrimitiveComponent Object Reference") (OtherActor :type "Actor Object Reference") (OtherComp :type "PrimitiveComponent Object Reference") (OtherBodyIndex :type Integer))
  (set `self.IsInInteractableRange` false)
  (if (== OtherActor (`GameplayStatics.GetPlayerCharacter` 0))
    (`Widget.RemoveFromParent` (`self.PromptUI`))))

(event `/Game/Blueprint/BPI_Interactable.Interact`
  (bind _returnvalue (`GameplayStatics.GetPlayerController` 0))
  (if (`self.IsInInteractableRange`)
    (`WidgetBlueprintLibrary.SetInputMode_UIOnlyEx` _returnvalue null)
    (set `PlayerController.bShowMouseCursor` true _returnvalue)
    (`UserWidget.AddToViewport` (`self.PasswordPadUI`) 0)))

(event `UnlockSecondDoor`
  (`self.K2_DestroyActor` (`self.PasswordDoor`)))

(fn `UserConstructionScript`)