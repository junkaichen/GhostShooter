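; BP_Enemy is an enemy Blueprint with a melee attack against the first-person player character.
; Its Attack event sphere-traces a short distance ahead for pawns and continues only if the hit actor is a BP_FirstPersonCharacter.
; On such a hit it plays the attack montage and applies damage at once, rather than timing the damage to the animation.
; The remaining events and the construction script are empty.
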(event `Attack`
  (bind _returnvalue (`self.K2_GetActorLocation`))
  ;[1 1 1] C4
  (bind (_outhit _returnvalue_2) (`KismetSystemLibrary.SphereTraceSingleForObjects` _returnvalue (+ _returnvalue (* (`KismetMathLibrary.GetForwardVector` (`self.K2_GetActorRotation`)) 250.0)) 120.0 (`|MakeArray` "ObjectTypeQuery3" :!type "EObjectTypeQuery Enum")))
  (if _returnvalue_2
    (bind (_bblockinghit _binitialoverlap _time _distance _location _impactpoint _normal _impactnormal _physmat _hitactor) (`GameplayStatics.BreakHitResult` _outhit))
    (cast `/Game/FirstPerson/Blueprints/BP_FirstPersonCharacter` _hitactor)
    (`self.PlayAnimMontage` "/Game/Animations/AM_Attack.AM_Attack")
    (`GameplayStatics.ApplyDamage` _hitactor 10.0)))

(fn `UserConstructionScript`)