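; Enemy spawner actor that spawns waves of enemies at its own transform, starting when play begins.
; Each Waves entry maps enemy classes to spawn counts and holds the delay before the next wave.
; SpawnEnemy waits, spawns every enemy in the current wave, then advances the wave number and calls itself with that delay while the pre-increment index is below the wave count.
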(event `SpawnEnemy`
  (params (DelayTime :type "Float (double-precision)"))
  (bind _output (`|GetArrayItem` (`self.Waves`) (`self.CurrentWaveNumber`)))
  (`KismetSystemLibrary.Delay` DelayTime)
  (set `self.Delay` (`.NextWaveTime_6_73ED6F9E48F121BB60E4428A755EE75B` (break `/Game/Blueprint/Wave` _output)))
  (bind _keys (`BlueprintMapLibrary.Map_Keys` (break `/Game/Blueprint/EnemyWaveInfo` (break `/Game/Blueprint/Wave` _output))))
  (for _array_element _keys
    (for _ (range (`BlueprintMapLibrary.Map_Find` (break `/Game/Blueprint/EnemyWaveInfo` (break `/Game/Blueprint/Wave` _output)) _array_element))
      (`|SpawnActorFromClass` _array_element (`self.GetTransform`) "AdjustIfPossibleButAlwaysSpawn" "MultiplyWithRoot" null null)))
  (if (< (`self.CurrentWaveNumber`) (`KismetArrayLibrary.Array_Length` (`self.Waves`)))
    (`/Engine/EditorBlueprintResources/StandardMacros.IncrementInt` (`self.CurrentWaveNumber`)
      (:`  `
        (`self.SpawnEnemy` (`self.Delay`))))))

(event `self.ReceiveBeginPlay`
  (`self.SpawnEnemy` 0.0))

(fn `UserConstructionScript`)