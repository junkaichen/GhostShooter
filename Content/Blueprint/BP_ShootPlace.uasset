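; BP_ShootPlace is an actor that generates and tracks a random four-digit password, apparently for a clue-based puzzle.
; On BeginPlay it builds CorrectPassword from random nonzero digits and prints it on screen.
; GetCurrentDigit hands out the digits in order, advancing a clue index.
; GetIndexFromNumber maps a digit to its position, flagging matches in HasBeenDisplay so repeated digits resolve to separate slots.
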(event `self.ReceiveBeginPlay`
  (for _ (range 4)
    (set `self.CorrectPassword` (`KismetStringLibrary.Concat_StrStr` (`self.CorrectPassword`) (`KismetStringLibrary.Conv_IntToString` (`KismetMathLibrary.RandomIntegerInRange` 1 9)))))
  (`KismetSystemLibrary.PrintString` (`self.CorrectPassword`) true true (struct :`G` 0.66 :`B` 1.0 :`A` 1.0) 10.0))

(fn `GetCurrentDigit`
  (returns (CurrentDigit :type String))
  (locals (CurrentIndex :type Integer))
  (if (< (`self.CurrentClueIndex`) 4)
    (bind _output_get (set `local.CurrentIndex` (`self.CurrentClueIndex`)))
    (`/Engine/EditorBlueprintResources/StandardMacros.IncrementInt` (`self.CurrentClueIndex`)
      (:`  `
        (return (`|GetArrayItem` (`KismetStringLibrary.GetCharacterArrayFromString` (`self.CorrectPassword`)) _output_get))))))

(fn `GetIndexFromNumber`
  (params (TargetChar :type String))
  (returns (Index :type Integer))
  (locals (TargetIndex :type Integer))
  (bind _hasbeendisplay (`self.HasBeenDisplay`))
  (for (_array_element _array_index) (`KismetStringLibrary.GetCharacterArrayFromString` (`self.CorrectPassword`))
    (if (`KismetStringLibrary.EqualEqual_StrStr` _array_element TargetChar)
      (if (not (`|GetArrayItem` _hasbeendisplay _array_index))
        (`KismetArrayLibrary.Array_Set` _hasbeendisplay _array_index true)
        (set `local.TargetIndex` _array_index)
        (break))))
  (return (`local.TargetIndex`)))

(fn `UserConstructionScript`)